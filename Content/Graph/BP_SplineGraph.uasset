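; Spline graph actor that lets the player start climbing along an ordered set of splines from an entry trigger.
; Overlapping EntryPoint sets IsInTrigger and caches the BP_Player; any end overlap clears the flag.
; EnterGraph calls the player's StartClimb when the flag is set and IsGround is false, passing the first spline, spline order, entry point and entry movement.
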(event OnComponentBeginOverlap(EntryPoint)
  (params (OverlappedComponent :type Primitive%20Component%20Object%20Reference) (OtherActor :type Actor%20Object%20Reference) (OtherComp :type Primitive%20Component%20Object%20Reference) (OtherBodyIndex :type Integer) (bFromSweep :type Boolean) (SweepResult :type Hit%20Result%20Structure%20%28by%20ref%29))
  (Variables|Default|SetIsInTrigger true)
  (bind _asbp_player (Utilities|Casting|CastToBP_Player OtherActor))
  (Variables|Default|SetPlayer _asbp_player))

(event OnComponentEndOverlap(EntryPoint)
  (params (OverlappedComponent :type Primitive%20Component%20Object%20Reference) (OtherActor :type Actor%20Object%20Reference) (OtherComp :type Primitive%20Component%20Object%20Reference) (OtherBodyIndex :type Integer))
  (Variables|Default|SetIsInTrigger false))

(event Custom|EnterGraph
  (bind _splineorder (Variables|Default|GetSplineOrder))
  (if (not (Variables|Default|GetIsGround))
    (if (Variables|Default|GetIsInTrigger)
      (Default|StartClimb (Variables|Default|GetPlayer) (Variables|/Game/Graph/BP_Spline.BP_Spline_C|GetSpline (Utilities|Array|Get(acopy) _splineorder)) _splineorder (Variables|Default|GetEntryPoint) (Variables|Default|GetEntryStartMovement)))))

(event EventBeginPlay)

(event Collision|EventActorBeginOverlap
  (params (OtherActor :type Actor%20Object%20Reference)))

(event EventTick
  (params (DeltaSeconds :type Float%20%28single-precision%29)))

(fn ConstructionScript)
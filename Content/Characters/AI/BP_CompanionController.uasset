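; BP_CompanionController is the AI controller for a companion character, running the BT_Companion behavior tree on possession.
; AI perception updates that sense a Player-tagged actor store it in the Blackboard as CompanionActor and set HasLineOfSight.
; Any other perception update starts a LineOfSightTimer delay that clears both keys, giving a grace period that a fresh player sighting cancels.
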(event OnTargetPerceptionUpdated(AIPerception)
  (params (Actor :type Actor%20Object%20Reference) (Stimulus :type AI%20Stimulus%20Structure))
  (bind _blackboard (Variables|Default|GetBlackboard))
  (bind _output_get (Variables|Default|SetPlayerActor Actor))
  (if (and (Actor|ActorHasTag _output_get "Player") (.bSuccessfullySensed (Utilities|Struct|BreakAIStimulus Stimulus)))
    (Utilities|Time|ClearandInvalidateTimerbyHandle (Variables|Default|GetCompanionTimer))
    (AI|Components|Blackboard|SetValueasBool _blackboard (Variables|Default|GetHasLineOfSight) true)
    (AI|Components|Blackboard|SetValueasObject _blackboard (Variables|Default|GetCompanionActor) (Variables|Default|GetPlayerActor))
    (else
      (bind _returnvalue (Utilities|Time|SetTimerbyEvent (delegate Custom|StartCompanionTimer) (Variables|Default|GetLineOfSightTimer)))
      (Variables|Default|SetCompanionTimer _returnvalue))))

(event Custom|StartCompanionTimer
  (bind _blackboard (Variables|Default|GetBlackboard))
  (AI|Components|Blackboard|SetValueasBool _blackboard (Variables|Default|GetHasLineOfSight) false)
  (AI|Components|Blackboard|SetValueasObject _blackboard (Variables|Default|GetCompanionActor) 0))

(event EventBeginPlay)

(event EventTick
  (params (DeltaSeconds :type Float%20%28single-precision%29)))

(event EventPossess
  (params (PossessedPawn :type Pawn%20Object%20Reference))
  (AI|RunBehaviorTree "/Game/Characters/AI/BT_Companion.BT_Companion"))

(fn ConstructionScript)
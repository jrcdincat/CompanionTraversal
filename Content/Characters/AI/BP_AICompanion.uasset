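; AI companion character that travels a pathfound route through a node graph along the splines linking the nodes.
; BeginPlay gets a path between two hardcoded test nodes, then selects each leg's spline and direction from the current node's spline maps.
; A timeline, rate-scaled by spline length and walk speed, feeds moving AIMoveTo goals along the spline.
; Once the timeline finishes, a looping timer advances the path whenever velocity is zero, gated by a DoOnce.
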(event Custom|DistanceCheck
  (bind _index (Variables|Default|GetIndex))
  (bind _traversalpath (Variables|Default|GetTraversalPath))
  (bind _graph (Variables|Default|GetGraph))
  (bind _output (Utilities|Array|Get(acopy) _traversalpath _index))
  (bind _value (Utilities|Map|Find _graph _output))
  (if (Math|Vector|VectorIsZero (Transformation|GetVelocity))
    (Variables|Default|SetCurrentNode _value)
    (Utilities|FlowControl|DoOnce false :!label _label
      (:Completed
        (if (< (Variables|Default|GetIndex) (- (Utilities|Array|Length (Variables|Default|GetTraversalPath)) 1))
          (bind _result (Math|Integer|IncrementInt (Variables|Default|GetIndex))
            (:%20%20
              (Development|PrintString (Utilities|String|ToString(Integer) _result))
              (Utilities|FlowControl|Sequence
                (:then_0
                  (if (.ReturnValue (Utilities|Map|Find (Variables|/Script/CompanionTraversal.AINode|GetnodeToSplineMap (Variables|Default|GetCurrentNode)) _value))
                    (bind _asbp_spline (Utilities|Casting|CastToBP_Spline (.Value (Utilities|Map|Find (Variables|/Script/CompanionTraversal.AINode|GetnodeToSplineMap (Variables|Default|GetCurrentNode)) _value))))
                    (bind _output_get (Variables|Default|SetTraverseSpline (Actor|GetComponentbyClass _asbp_spline "/Script/Engine.SplineComponent")))
                    (Variables|Default|SetDuration (/ (Spline|GetSplineLength _output_get) (Variables|/Script/Engine.CharacterMovementComponent|GetMaxWalkSpeed (Variables|Character|GetCharacterMovement))))
                    (Variables|Default|SetIsReverse true)
                    (elif (.ReturnValue (Utilities|Map|Find (Variables|/Script/CompanionTraversal.AINode|GetreferenceNodeToSplineMap (Variables|Default|GetCurrentNode)) _value))
                      (bind _asbp_spline_2 (Utilities|Casting|CastToBP_Spline (.Value (Utilities|Map|Find (Variables|/Script/CompanionTraversal.AINode|GetreferenceNodeToSplineMap (Variables|Default|GetCurrentNode)) _value))))
                      (bind _output_get_2 (Variables|Default|SetTraverseSpline (Actor|GetComponentbyClass _asbp_spline_2 "/Script/Engine.SplineComponent")))
                      (Variables|Default|SetDuration (/ (Spline|GetSplineLength _output_get_2) (Variables|/Script/Engine.CharacterMovementComponent|GetMaxWalkSpeed (Variables|Character|GetCharacterMovement))))
                      (Variables|Default|SetIsReverse false))))
                (:then_1
                  (Components|Timeline|SetPlayRate (Variables|Default|GetMoveTimeline) (/ 1.0 (Variables|Default|GetDuration)))
                  (bind _alpha (Timeline|MoveTimeline PlayFromStart)
                    (:Update
                      (Variables|Default|SetAlpha _alpha)
                      (if (Variables|Default|GetIsReverse)
                        (AI|AIMoveTo (AI|GetAIController self) (Spline|GetLocationatDistanceAlongSpline (Variables|Default|GetTraverseSpline) (Math|Float|Lerp (Spline|GetSplineLength (Variables|Default|GetTraverseSpline)) 0.0 (Variables|Default|GetAlpha)) "World") 0 -1.0 "Default" "Default" true true
                          (:then
                            (goto _label Reset)))
                        (else
                          (AI|AIMoveTo (AI|GetAIController self) (Spline|GetLocationatDistanceAlongSpline (Variables|Default|GetTraverseSpline) (Math|Float|Lerp 0.0 (Spline|GetSplineLength (Variables|Default|GetTraverseSpline)) (Variables|Default|GetAlpha)) "World") 0 -1.0 "Default" "Default" true true
                            (:then
                              (goto _label Reset))))))
                    (:Finished
                      (Utilities|FlowControl|DoOnce false
                        (:Completed
                          (CallFunction|StartDistanceCheckTimer))))))))))))))

(event Custom|StartDistanceCheckTimer
  (Utilities|Time|SetTimerbyEvent (delegate Custom|DistanceCheck) 1.0 true))

(event EventBeginPlay
  (bind _returnvalue (Class|AIBase|PathFindingTest 0 6))
  (Variables|Default|SetTraversalPath _returnvalue)
  (Variables|Default|SetCurrentNode (.Value (Utilities|Map|Find (Variables|Default|GetGraph) (Utilities|Array|Get(acopy) (Variables|Default|GetTraversalPath)))))
  (Utilities|FlowControl|Sequence
    (:then_0
      (if (.ReturnValue (Utilities|Map|Find (Variables|/Script/CompanionTraversal.AINode|GetnodeToSplineMap (Variables|Default|GetCurrentNode)) (.Value (Utilities|Map|Find (Variables|Default|GetGraph) (Utilities|Array|Get(acopy) (Variables|Default|GetTraversalPath) (Variables|Default|GetIndex))))))
        (bind _asbp_spline (Utilities|Casting|CastToBP_Spline (.Value (Utilities|Map|Find (Variables|/Script/CompanionTraversal.AINode|GetnodeToSplineMap (Variables|Default|GetCurrentNode)) (.Value (Utilities|Map|Find (Variables|Default|GetGraph) (Utilities|Array|Get(acopy) (Variables|Default|GetTraversalPath) (Variables|Default|GetIndex))))))))
        (bind _output_get (Variables|Default|SetTraverseSpline (Actor|GetComponentbyClass _asbp_spline "/Script/Engine.SplineComponent")))
        (Variables|Default|SetDuration (/ (Spline|GetSplineLength _output_get) (Variables|/Script/Engine.CharacterMovementComponent|GetMaxWalkSpeed (Variables|Character|GetCharacterMovement))))
        (Variables|Default|SetIsReverse true)
        (elif (.ReturnValue (Utilities|Map|Find (Variables|/Script/CompanionTraversal.AINode|GetreferenceNodeToSplineMap (Variables|Default|GetCurrentNode)) (.Value (Utilities|Map|Find (Variables|Default|GetGraph) (Utilities|Array|Get(acopy) (Variables|Default|GetTraversalPath) (Variables|Default|GetIndex))))))
          (bind _asbp_spline_2 (Utilities|Casting|CastToBP_Spline (.Value (Utilities|Map|Find (Variables|/Script/CompanionTraversal.AINode|GetreferenceNodeToSplineMap (Variables|Default|GetCurrentNode)) (.Value (Utilities|Map|Find (Variables|Default|GetGraph) (Utilities|Array|Get(acopy) (Variables|Default|GetTraversalPath) (Variables|Default|GetIndex))))))))
          (bind _output_get_2 (Variables|Default|SetTraverseSpline (Actor|GetComponentbyClass _asbp_spline_2 "/Script/Engine.SplineComponent")))
          (Variables|Default|SetDuration (/ (Spline|GetSplineLength _output_get_2) (Variables|/Script/Engine.CharacterMovementComponent|GetMaxWalkSpeed (Variables|Character|GetCharacterMovement))))
          (Variables|Default|SetIsReverse false))))
    (:then_1
      (Components|Timeline|SetPlayRate (Variables|Default|GetMoveTimeline) (/ 1.0 (Variables|Default|GetDuration)))
      (bind _alpha (Timeline|MoveTimeline PlayFromStart)
        (:Update
          (Variables|Default|SetAlpha _alpha)
          (if (Variables|Default|GetIsReverse)
            (AI|AIMoveTo (AI|GetAIController self) (Spline|GetLocationatDistanceAlongSpline (Variables|Default|GetTraverseSpline) (Math|Float|Lerp (Spline|GetSplineLength (Variables|Default|GetTraverseSpline)) 0.0 (Variables|Default|GetAlpha)) "World") 0 -1.0 "Default" "Default" true true
              (:then
                (Utilities|FlowControl|DoOnce false) ; enters at Reset
              ))
            (else
              (AI|AIMoveTo (AI|GetAIController self) (Spline|GetLocationatDistanceAlongSpline (Variables|Default|GetTraverseSpline) (Math|Float|Lerp 0.0 (Spline|GetSplineLength (Variables|Default|GetTraverseSpline)) (Variables|Default|GetAlpha)) "World") 0 -1.0 "Default" "Default" true true
                (:then
                  (Utilities|FlowControl|DoOnce false) ; enters at Reset
                )))))
        (:Finished
          (Utilities|FlowControl|DoOnce false
            (:Completed
              (CallFunction|StartDistanceCheckTimer))))))))

(fn ConstructionScript)

(fn UpdateWalkSpeed
  (params (NewWalkSpeed :type Float%20%28double-precision%29))
  (Variables|/Script/Engine.CharacterMovementComponent|SetMaxWalkSpeed (Variables|Character|GetCharacterMovement) NewWalkSpeed))

(fn TraverseGraph)